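; First-person character that carries two BP_Gun child actors, one in hand and one on the back, handling movement, firing, reload, aim, fire mode and laser input.
; A state variable gates actions across idle, aiming, reloading, swapping and running.
; ABP_QC anim notifies drive magazine handling, reload completion and the put, swap, draw sequence.
; Lower-body and first-person meshes each hide bones, and running doubles walk speed while moving forward.
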(event `self.ReceiveBeginPlay`
  (`SkinnedMeshComponent.HideBoneByName` (`self.LowerBody`) "spine_02" "PBO_None")
  (`SkinnedMeshComponent.HideBoneByName` (`self.FirstPerson`) "neck_01" "PBO_None")
  (bind _asbp_gun (cast `/Game/_DEV/Gun/BP_Gun` (`ChildActorComponent.ChildActor` (`self.WeaponInHand`))))
  (set `self.GunInHand` _asbp_gun)
  (bind _asbp_gun_2 (cast `/Game/_DEV/Gun/BP_Gun` (`ChildActorComponent.ChildActor` (`self.WeaponInBack`))))
  (set `self.GunInBack` _asbp_gun_2)
  (`self.BindAnimNotifies`))

(event `self.ReceiveTick`
  (params (DeltaSeconds :type "Float (single-precision)"))
  (`self.TickRun`))

(event `EnhancedInput|/Game/_DEV/Input/IA_GunMoveForward`
  (params (ActionValue :type "Float (double-precision)") (ElapsedSeconds :type "Float (double-precision)") (TriggeredSeconds :type "Float (double-precision)") (InputAction :type "InputAction Object Reference" :default "/Game/_DEV/Input/IA_GunMoveForward.IA_GunMoveForward"))
  (:`Triggered`
    (bind _output_get (set `self.MoveForwardValue` ActionValue))
    (`self.AddMovementInput` (`KismetMathLibrary.GetForwardVector` (`self.K2_GetActorRotation`)) _output_get)))

(event `EnhancedInput|/Game/_DEV/Input/IA_GunTurnPitch`
  (params (ActionValue :type "Float (double-precision)") (ElapsedSeconds :type "Float (double-precision)") (TriggeredSeconds :type "Float (double-precision)") (InputAction :type "InputAction Object Reference" :default "/Game/_DEV/Input/IA_GunTurnPitch.IA_GunTurnPitch"))
  (:`Triggered`
    (`self.AddControllerPitchInput` ActionValue)))

(event `EnhancedInput|/Game/_DEV/Input/IA_GunMoveRight`
  (params (ActionValue :type "Float (double-precision)") (ElapsedSeconds :type "Float (double-precision)") (TriggeredSeconds :type "Float (double-precision)") (InputAction :type "InputAction Object Reference" :default "/Game/_DEV/Input/IA_GunMoveRight.IA_GunMoveRight"))
  (:`Triggered`
    (`self.AddMovementInput` (`KismetMathLibrary.GetRightVector` (`self.K2_GetActorRotation`)) ActionValue)))

(event `EnhancedInput|/Game/_DEV/Input/IA_GunTurnYaw`
  (params (ActionValue :type "Float (double-precision)") (ElapsedSeconds :type "Float (double-precision)") (TriggeredSeconds :type "Float (double-precision)") (InputAction :type "InputAction Object Reference" :default "/Game/_DEV/Input/IA_GunTurnYaw.IA_GunTurnYaw"))
  (:`Triggered`
    (`self.AddControllerYawInput` ActionValue)))

(event `EnhancedInput|/Game/_DEV/Input/IA_GunFire`
  (params (ActionValue :type Boolean) (ElapsedSeconds :type "Float (double-precision)") (TriggeredSeconds :type "Float (double-precision)") (InputAction :type "InputAction Object Reference" :default "/Game/_DEV/Input/IA_GunFire.IA_GunFire"))
  (bind _guninhand (`self.GunInHand`))
  (:`Triggered`
    (switch `/Game/_DEV/Gameplay/StateOfCharacter` (`self.State`)
      (:`NewEnumerator0`
        _)
      (:`NewEnumerator1`
        _))
    (if ActionValue
      (`/Game/_DEV/Gun/BP_Gun.FirePressed` _guninhand)
      (else
        (`/Game/_DEV/Gun/BP_Gun.FireReleased` _guninhand)))))

(event `EnhancedInput|/Game/_DEV/Input/IA_GunReload`
  (params (ActionValue :type Boolean) (ElapsedSeconds :type "Float (double-precision)") (TriggeredSeconds :type "Float (double-precision)") (InputAction :type "InputAction Object Reference" :default "/Game/_DEV/Input/IA_GunReload.IA_GunReload"))
  (bind _guninhand (`self.GunInHand`))
  (:`Triggered`
    (switch `/Game/_DEV/Gameplay/StateOfCharacter` (`self.State`)
      (:`NewEnumerator0`
        (if (`/Game/_DEV/Gun/BP_Gun.CanReload` _guninhand)
          (`/Game/_DEV/Gun/BP_Gun.ReloadStart` _guninhand)
          (`/Game/_DEV/Gun/BP_Gun.FireReleased` _guninhand)
          (set `self.State` "NewEnumerator2"))))))

(event `EnhancedInput|/Game/_DEV/Input/IA_GunSwapMain`
  (params (ActionValue :type Boolean) (ElapsedSeconds :type "Float (double-precision)") (TriggeredSeconds :type "Float (double-precision)") (InputAction :type "InputAction Object Reference" :default "/Game/_DEV/Input/IA_GunSwapMain.IA_GunSwapMain"))
  (bind _guninhand (`self.GunInHand`))
  (:`Triggered`
    (switch `/Game/_DEV/Gameplay/StateOfCharacter` (`self.State`)
      (:`NewEnumerator0`
        (switch `/Game/_DEV/Gun/UseTypeOfGun` (`/Game/_DEV/Gun/BP_Gun.GetUseType` _guninhand)
          (:`NewEnumerator1`
            (`/Game/_DEV/Gun/BP_Gun.PutThis` _guninhand)
            (set `self.State` "NewEnumerator3")))))))

(event `EnhancedInput|/Game/_DEV/Input/IA_GunSwapSub`
  (params (ActionValue :type Boolean) (ElapsedSeconds :type "Float (double-precision)") (TriggeredSeconds :type "Float (double-precision)") (InputAction :type "InputAction Object Reference" :default "/Game/_DEV/Input/IA_GunSwapSub.IA_GunSwapSub"))
  (bind _guninhand (`self.GunInHand`))
  (:`Triggered`
    (switch `/Game/_DEV/Gameplay/StateOfCharacter` (`self.State`)
      (:`NewEnumerator0`
        (switch `/Game/_DEV/Gun/UseTypeOfGun` (`/Game/_DEV/Gun/BP_Gun.GetUseType` _guninhand)
          (:`NewEnumerator0`
            (`/Game/_DEV/Gun/BP_Gun.PutThis` _guninhand)
            (set `self.State` "NewEnumerator3")))))))

(event `EnhancedInput|/Game/_DEV/Input/IA_GunFireMode`
  (params (ActionValue :type Boolean) (ElapsedSeconds :type "Float (double-precision)") (TriggeredSeconds :type "Float (double-precision)") (InputAction :type "InputAction Object Reference" :default "/Game/_DEV/Input/IA_GunFireMode.IA_GunFireMode"))
  (:`Triggered`
    (switch `/Game/_DEV/Gameplay/StateOfCharacter` (`self.State`)
      (:`NewEnumerator0`
        (`/Game/_DEV/Gun/BP_Gun.ChangeFireMode` (`self.GunInHand`))))))

(event `EnhancedInput|/Game/_DEV/Input/IA_ToggleLaser`
  (params (ActionValue :type Boolean) (ElapsedSeconds :type "Float (double-precision)") (TriggeredSeconds :type "Float (double-precision)") (InputAction :type "InputAction Object Reference" :default "/Game/_DEV/Input/IA_ToggleLaser.IA_ToggleLaser"))
  (:`Triggered`
    (switch `/Game/_DEV/Gameplay/StateOfCharacter` (`self.State`)
      (:`NewEnumerator0`
        (`/Game/_DEV/Gun/BP_Gun.ToggleLaser` (`self.GunInHand`))))))

(event `EnhancedInput|/Game/_DEV/Input/IA_GunAim`
  (params (ActionValue :type Boolean) (ElapsedSeconds :type "Float (double-precision)") (TriggeredSeconds :type "Float (double-precision)") (InputAction :type "InputAction Object Reference" :default "/Game/_DEV/Input/IA_GunAim.IA_GunAim"))
  (:`Triggered`
    (`self.ToggleAim`)))

(event `EnhancedInput|/Game/_DEV/Input/IA_GunRun`
  (params (ActionValue :type Boolean) (ElapsedSeconds :type "Float (double-precision)") (TriggeredSeconds :type "Float (double-precision)") (InputAction :type "InputAction Object Reference" :default "/Game/_DEV/Input/IA_GunRun.IA_GunRun"))
  (:`Triggered`
    (set `self.IsRunPressed` ActionValue)))

(fn `BindAnimNotifies`
  (bind _asabp_qc (cast `/Game/_DEV/Character/QC/Animation/ABP_QC` (`SkeletalMeshComponent.GetAnimInstance` (`self.FirstPerson`))))
  (add `/Game/_DEV/Character/QC/Animation/ABP_QC.OnReloadComplete` _asabp_qc (`|CreateDelegate` :!event `OnReloadComplete`))
  (add `/Game/_DEV/Character/QC/Animation/ABP_QC.OnMagazieDetached` _asabp_qc (`|CreateDelegate` :!event `OnMagazineDetached`))
  (add `/Game/_DEV/Character/QC/Animation/ABP_QC.OnMagazineAttached` _asabp_qc (`|CreateDelegate` :!event `OnMagazineAttached`))
  (add `/Game/_DEV/Character/QC/Animation/ABP_QC.OnPutComplete` _asabp_qc (`|CreateDelegate` :!event `OnPutComplete`))
  (add `/Game/_DEV/Character/QC/Animation/ABP_QC.OnDrawComplete` _asabp_qc (`|CreateDelegate` :!event `OnDrawComplete`)))

(fn `CanRun`
  (returns (ReturnValue :type Boolean))
  (return (and (> (`self.MoveForwardValue`) 0.0) (`self.IsRunPressed`))))

(fn `GetGunInHand`
  (returns (Result :type "/Game/_DEV/Gun/BP_Gun Object Reference"))
  (return (`self.GunInHand`)))

(fn `GetSocketTransform`
  (params (InSocketName :type Name))
  (returns (ReturnValue :type "Transform Structure"))
  (return (`SceneComponent.GetSocketTransform` (`self.FirstPerson`) InSocketName "RTS_World")))

(fn `GetSpeed`
  (returns (ReturnValue :type "Float (double-precision)"))
  (return (`KismetMathLibrary.VSize` (`self.GetVelocity`))))

(fn `GetState`
  (returns (State :type "/Game/_DEV/Gameplay/StateOfCharacter Enum"))
  (return (`self.State`)))

(fn `IsAiming`
  (returns (ReturnValue :type Boolean))
  (return (`|EnumEquality` (`self.State`) "NewEnumerator1")))

(fn `OnDrawComplete`
  (set `self.State` "NewEnumerator0"))

(fn `OnMagazineAttached`
  (`/Game/_DEV/Gun/BP_Gun.AttachMagazine` (`self.GunInHand`)))

(fn `OnMagazineDetached`
  (`/Game/_DEV/Gun/BP_Gun.DetachMagazine` (`self.GunInHand`)))

(fn `OnPutComplete`
  (`self.SwapGun`)
  (`/Game/_DEV/Gun/BP_Gun.DrawThis` (`self.GunInHand`)))

(fn `OnReloadComplete`
  (set `self.State` "NewEnumerator0")
  (`/Game/_DEV/Gun/BP_Gun.ReloadComplete` (`self.GunInHand`)))

(fn `PlayMontage`
  (params (Animation :type "AnimMontage Object Reference"))
  (bind _asabp_qc (cast `/Game/_DEV/Character/QC/Animation/ABP_QC` (`SkeletalMeshComponent.GetAnimInstance` (`self.FirstPerson`))))
  (`AnimInstance.Montage_Play` _asabp_qc (`local.Animation`) 1.0 "MontageLength" 0.0 true))

(fn `SwapGun`
  (if (not (`/Game/_DEV/Gun/BP_Gun.IsBusy` (`self.GunInHand`)))
    (set `self.WillBeDrawn` (`self.GunInBack`))
    (set `self.WillBePut` (`self.GunInHand`))
    (`self.K2_AttachToComponent` (`self.WillBeDrawn`) (`self.WeaponInHand`) "None" "KeepRelative" "KeepRelative" "KeepRelative" true)
    (`self.K2_AttachToComponent` (`self.WillBePut`) (`self.WeaponInBack`) "None" "KeepRelative" "KeepRelative" "KeepRelative" true)
    (set `self.GunInHand` (`self.WillBeDrawn`))
    (set `self.GunInBack` (`self.WillBePut`))
    (`SceneComponent.K2_SetRelativeTransform` (`self.WeaponInHand`) (`/Game/_DEV/Gun/BP_Gun.GetHandTransform` (`self.GunInHand`)) false false)))

(fn `TickRun`
  (bind _charactermovement (`self.CharacterMovement`))
  (bind _charactermovement_2 (`self.CharacterMovement`))
  (if (`self.CanRun`)
    (switch `/Game/_DEV/Gameplay/StateOfCharacter` (`self.State`)
      (:`NewEnumerator0`
        (set `self.State` "NewEnumerator4")
        (set `CharacterMovementComponent.MaxWalkSpeed` (* (`CharacterMovementComponent.MaxWalkSpeed` _charactermovement_2) 2.0) _charactermovement_2)))
    (else
      (switch `/Game/_DEV/Gameplay/StateOfCharacter` (`self.State`)
        (:`NewEnumerator4`
          (set `self.State` "NewEnumerator0")
          (set `CharacterMovementComponent.MaxWalkSpeed` (* (`CharacterMovementComponent.MaxWalkSpeed` _charactermovement) 0.5) _charactermovement))))))

(fn `ToggleAim`
  (bind _guninhand (`self.GunInHand`))
  (if (`/Game/_DEV/Gun/BP_Gun.IsBusy` _guninhand)
    _
    (elif (`/Game/_DEV/Gun/BP_Gun.DoesSupportAim` _guninhand)
      (switch `/Game/_DEV/Gameplay/StateOfCharacter` (`self.State`)
        (:`NewEnumerator0`
          (set `self.State` "NewEnumerator1"))
        (:`NewEnumerator1`
          (set `self.State` "NewEnumerator0"))))))

(fn `UserConstructionScript`)