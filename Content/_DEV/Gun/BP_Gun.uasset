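; BP_Gun is a weapon actor with semi and full auto fire modes, ammo, reloading, a laser pointer toggle and getters for weapon state.
; Fire spawns a BP_Bullet at the muzzle, re-arming itself by timer in full auto until release, or plays a dry-fire sound when empty.
; Reload, draw and put-away play montages on the player's BP_GunCharacter.
; The mesh's magazine bone is hidden, and detach/attach toggle a separate Magazine component with sounds.
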(event `self.ReceiveBeginPlay`
  (`SkinnedMeshComponent.HideBoneByName` (`self.Gun`) "b_gun_mag" "PBO_None"))

(fn `AttachMagazine`
  (`SceneComponent.SetVisibility` (`self.Magazine`) true false)
  (`GameplayStatics.PlaySoundAtLocation` (`self.AttachMagazineSound`) (`SceneComponent.K2_GetComponentLocation` (`self.Magazine`)) (struct) 1.0 1.0 0.0 null null null null))

(fn `CanReload`
  (returns (Result :type Boolean))
  (return (< (`self.RemainingBullet`) (`self.MaxRemainingBullet`))))

(fn `ChangeFireMode`
  (`GameplayStatics.PlaySoundAtLocation` (`self.FireModeSound`) (`SceneComponent.K2_GetComponentLocation` (`self.Gun`)) (struct) 1.0 1.0 0.0 null null null null)
  (switch `/Game/_DEV/Gun/FireModeOfGun` (`self.FireMode`)
    (:`NewEnumerator0`
      (set `self.FireMode` "NewEnumerator1"))
    (:`NewEnumerator1`
      (set `self.FireMode` "NewEnumerator0"))))

(fn `DetachMagazine`
  (`SceneComponent.SetVisibility` (`self.Magazine`) false false)
  (`GameplayStatics.PlaySoundAtLocation` (`self.DetachMagazineSound`) (`SceneComponent.K2_GetComponentLocation` (`self.Magazine`)) (struct) 1.0 1.0 0.0 null null null null))

(fn `DoesSupportAim`
  (returns (SuportAim :type Boolean))
  (locals (NewLocalVar :type Boolean :default false))
  (return (`self.SuportAim`)))

(fn `DrawThis`
  (bind _asbp_gun_character (cast `/Game/_DEV/Gameplay/BP_GunCharacter` (`GameplayStatics.GetPlayerCharacter` 0)))
  (`/Game/_DEV/Gameplay/BP_GunCharacter.PlayMontage` _asbp_gun_character (`self.DrawAnim`)))

(fn `Fire`
  (if (> (`self.RemainingBullet`) 0)
    (`/Engine/EditorBlueprintResources/StandardMacros.DecrementInt` (`self.RemainingBullet`)
      (:`  `
        (`|ExecutionSequence`
          (:`then_0`
            (bind _returnvalue (`|SpawnActorFromClass` "/Game/_DEV/Gun/BP_Bullet.BP_Bullet_C" (`SceneComponent.K2_GetComponentToWorld` (`self.FrontOfGun`)) "Undefined" "MultiplyWithRoot" null null))
            (`/Game/_DEV/Gun/BP_Bullet.SetSpeed` _returnvalue 1000.0))
          (:`then_1`
            (switch `/Game/_DEV/Gun/FireModeOfGun` (`self.FireMode`)
              (:`NewEnumerator1`
                (bind _returnvalue_2 (`KismetSystemLibrary.K2_SetTimer` null "Fire" (`self.DurationPerFire`)))
                (set `self.TimeFire` _returnvalue_2))))
          (:`then_2`
            (`GameplayStatics.PlaySoundAtLocation` (`self.FireSound`) (`SceneComponent.K2_GetComponentLocation` (`self.FrontOfGun`)) (struct) 1.0 1.0 0.0 null null null null)))))
    (else
      (`GameplayStatics.PlaySoundAtLocation` (`self.DryFireSound`) (`SceneComponent.K2_GetComponentLocation` (`self.Gun`)) (struct) 1.0 1.0 0.0 null null null null))))

(fn `FirePressed`
  (set `self.IsFirePressed` true)
  (`self.Fire`))

(fn `FireReleased`
  (set `self.IsFirePressed` false)
  (`KismetSystemLibrary.K2_ClearAndInvalidateTimerHandle` (`self.TimeFire`)))

(fn `GetFireMode`
  (returns (Result :type "/Game/_DEV/Gun/FireModeOfGun Enum"))
  (return (`self.FireMode`)))

(fn `GetHandTransform`
  (returns (HandTransform :type "Transform Structure"))
  (return (`self.HandTransform`)))

(fn `GetMaxRemainBullets`
  (returns (Result :type Integer))
  (return (`self.MaxRemainingBullet`)))

(fn `GetRemainBullets`
  (returns (Result :type Integer))
  (return (`self.RemainingBullet`)))

(fn `GetUseType`
  (returns (Result :type "/Game/_DEV/Gun/UseTypeOfGun Enum"))
  (return (`self.UseType`)))

(fn `GetWeaponName`
  (returns (Result :type Name))
  (return (`self.WeaponName`)))

(fn `IsBusy`
  (returns (Result :type Boolean))
  (return (`self.IsFiring`)))

(fn `IsFiring`
  (returns (Resutl :type Boolean))
  (return (and (`self.IsFirePressed`) (`KismetSystemLibrary.K2_IsTimerActiveHandle` (`self.TimeFire`)))))

(fn `PutThis`
  (bind _asbp_gun_character (cast `/Game/_DEV/Gameplay/BP_GunCharacter` (`GameplayStatics.GetPlayerCharacter` 0)))
  (`/Game/_DEV/Gameplay/BP_GunCharacter.PlayMontage` _asbp_gun_character (`self.PutAnim`)))

(fn `ReloadComplete`
  (set `self.RemainingBullet` (`self.MaxRemainingBullet`))
  (`GameplayStatics.PlaySoundAtLocation` (`self.ReloadCompleteSound`) (`SceneComponent.K2_GetComponentLocation` (`self.Gun`)) (struct) 1.0 1.0 0.0 null null null null))

(fn `ReloadStart`
  (bind _asbp_gun_character (cast `/Game/_DEV/Gameplay/BP_GunCharacter` (`GameplayStatics.GetPlayerCharacter` 0)))
  (`/Game/_DEV/Gameplay/BP_GunCharacter.PlayMontage` _asbp_gun_character (`self.ReloadAnimation`)))

(fn `ToggleLaser`
  (bind _asbp_laser_pointer (cast `/Game/_DEV/Gun/BP_LaserPointer` (`ChildActorComponent.ChildActor` (`self.LaserPointer`))))
  (`/Game/_DEV/Gun/BP_LaserPointer.ShowLaserPointer` _asbp_laser_pointer))

(fn `UserConstructionScript`)